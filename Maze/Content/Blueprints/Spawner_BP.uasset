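; Spawner actor that creates Scarecrow_BP enemies at its own location in the Soul Maze game.
; SpawnScarecrow spawns the AI, plays a 2D sound and increments the bot count on SoulMazeGameMode.
; MoveAi shuffles three target references and prints the first one's name as debug output.
; The relocation to that target and the delayed repeat are disconnected, so the spawner never moves.
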(event Custom|Move%20Ai
  (Development|PrintString "Moved")
  (Variables|Default|SetSelected%20Destination (Utilities|Array|MakeArray (Variables|Default|GetTarget1) (Variables|Default|GetTarget2) (Variables|Default|GetTarget3)))
  (for _index (range 0 2)
    (Utilities|Array|Shuffle (Variables|Default|GetSelected%20Destination)))
  (Development|PrintString (Utilities|GetDisplayName (Utilities|Array|Get(acopy) (Variables|Default|GetSelected%20Destination)))))

(fn ConstructionScript)

(fn SpawnScarecrow
  (AI|SpawnAIFromClass "/Game/Ai/ScareCrow_Ai/Scarecrow_BP.Scarecrow_BP_C" 0 (Transformation|GetActorLocation) "0, 0, 0" false 0)
  (Audio|SpawnSound2D "/Game/Audio/Cropfield/species-lair-of-the-demonspawn-sound-effect-36157227.species-lair-of-the-demonspawn-sound-effect-36157227" 1.0 1.0 0.0 0)
  (bind _asthird_person_game_mode (Utilities|Casting|CastToSoulMazeGameMode (Game|GetGameMode)))
  (Math|Integer|IncrementInt (Variables|/Game/GameModes/SoulMazeGameMode.SoulMazeGameMode_C|GetNumberofBots _asthird_person_game_mode)))
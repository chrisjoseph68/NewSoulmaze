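; Portal actor for the SoulMaze game that acts as the level exit once all collectables are gathered.
; Overlapping its box checks the game mode's CollectablesLeft count.
; At zero, an overlapping ThirdPersonCharacter pauses the game, opens the EndGame widget and shows the mouse cursor.
; Otherwise any overlap shows a NoOrbs widget for a short delay, then removes it.
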(event OnComponentBeginOverlap(Box)
  (params (OverlappedComponent :type Primitive%20Component%20Object%20Reference) (OtherActor :type Actor%20Object%20Reference) (OtherComp :type Primitive%20Component%20Object%20Reference) (OtherBodyIndex :type Integer) (bFromSweep :type Boolean) (SweepResult :type Hit%20Result%20Structure%20%28by%20ref%29))
  (bind _asthird_person_game_mode (Utilities|Casting|CastToSoulMazeGameMode (Game|GetGameMode)))
  (if (== (Variables|/Game/GameModes/SoulMazeGameMode.SoulMazeGameMode_C|GetCollectables%20Left _asthird_person_game_mode) 0)
    (Utilities|Casting|CastToThirdPersonCharacter OtherActor)
    (Game|SetGamePaused true)
    (bind _returnvalue (UserInterface|CreateWidget "/Game/Ui/EndGAME.EndGame_C" (Game|GetPlayerController 0)))
    (UserInterface|Viewport|AddtoViewport _returnvalue 0)
    (Variables|/Script/Engine.PlayerController|SetbShowMouseCursor (Game|GetPlayerController 0) true)
    (else
      (bind _returnvalue_2 (UserInterface|CreateWidget "/Game/Ui/NoOrbs.NoOrbs_C"))
      (UserInterface|Viewport|AddtoViewport _returnvalue_2 0)
      (Utilities|FlowControl|Delay 1.0)
      (Widget|RemovefromParent _returnvalue_2))))

(fn ConstructionScript)
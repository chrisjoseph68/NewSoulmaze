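; Scarecrow enemy character that chases its behavior through a Scarecrow_Ai controller and can melee attack the player.
; On BeginPlay it passes its behavior tree and the player pawn to the controller, then spawns an actor attached to a mesh socket.
; Separate events play the attack montage and apply damage to the player.
; Sound and movement-stop nodes are left unconnected.
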(event Custom|DamagePlayer
  (Game|Damage|ApplyDamage (Variables|Default|GetPlayer) (Variables|Default|GetDamage) 0 self))

(event EventEnemyMeleeAttack
  (Animation|Montage|PlayMontage (Variables|Character|GetMesh) (Variables|Default|GetMontage%20to%20Play)))

(event EventBeginPlay
  (Utilities|FlowControl|Sequence
    (:then_0
      (bind _asscarecrow_ai (Utilities|Casting|CastToScarecrow_Ai (AI|GetAIController self)))
      (Default|SetupAI _asscarecrow_ai (Variables|Default|GetBT) (Game|Player|GetPlayerPawn 0)))
    (:then_1
      (bind _returnvalue (Game|SpawnActorfromClass (Variables|Default|GetClass) (Transformation|GetSocketTransform (Variables|Character|GetMesh) (Variables|Default|GetIn%20Socket%20Name) "RTS_World") "Undefined" 0 0))
      (Transformation|AttachComponentToComponent _returnvalue (Variables|Character|GetMesh) (Variables|Default|GetIn%20Socket%20Name) "SnapToTarget" "SnapToTarget" "SnapToTarget" false))))

(fn ConstructionScript)
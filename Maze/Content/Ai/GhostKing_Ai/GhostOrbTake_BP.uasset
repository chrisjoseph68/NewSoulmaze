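; Ghost orb hazard, filed with the Ghost King AI, that drains the player's light batteries on contact.
; When a ThirdPersonCharacter overlaps its TakeLight component, it lowers both FlashLighBattery and BlueLightBattery, then destroys itself after a short delay.
; Repeat overlaps during that delay drain again, as nothing guards the subtraction.
; An untouched orb removes itself after a timed lifetime started on BeginPlay.
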(event OnComponentBeginOverlap(TakeLight)
  (params (OverlappedComponent :type Primitive%20Component%20Object%20Reference) (OtherActor :type Actor%20Object%20Reference) (OtherComp :type Primitive%20Component%20Object%20Reference) (OtherBodyIndex :type Integer) (bFromSweep :type Boolean) (SweepResult :type Hit%20Result%20Structure%20%28by%20ref%29))
  (bind _asthird_person_character (Utilities|Casting|CastToThirdPersonCharacter OtherActor))
  (Variables|/Game/ThirdPersonBP/Blueprints/ThirdPersonCharacter.ThirdPersonCharacter_C|SetFlashLighBattery _asthird_person_character (- (Variables|/Game/ThirdPersonBP/Blueprints/ThirdPersonCharacter.ThirdPersonCharacter_C|GetFlashLighBattery _asthird_person_character) 1.0))
  (Variables|/Game/ThirdPersonBP/Blueprints/ThirdPersonCharacter.ThirdPersonCharacter_C|SetBlueLightBattery _asthird_person_character (- (Variables|/Game/ThirdPersonBP/Blueprints/ThirdPersonCharacter.ThirdPersonCharacter_C|GetBlueLightBattery _asthird_person_character) 1.0))
  (Utilities|FlowControl|Delay 2.0)
  (Actor|DestroyActor))

(event EventBeginPlay
  (|CallParentFunction)
  (Utilities|FlowControl|Delay 3e+01)
  (Actor|DestroyActor))

(fn ConstructionScript
  (|CallParentFunction))
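; GhostKing Blueprint that acts as an enemy spawner, repeatedly spawning waves of three actor classes: Enemy, Take and Teleport.
; BeginPlay starts three custom events, each spawning NumberOfEnemies copies of its class at the actor's transform.
; Each event calls itself again after a Delay, re-reading the transform, so waves continue with no count limit.
; Enemy and Teleport waves share SpawnDelay, while Take waves use SpawnDelay2.
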(event Custom|SpawnEnemy3
  (params (Teleport :type Actor%20Class%20Reference) (SpawnTransform :type Transform) (NumberOfEnemies :type Integer))
  (for _index (range 0 (- NumberOfEnemies 1))
    (Game|SpawnActorfromClass Teleport SpawnTransform "Undefined" 0 0))
  (Utilities|FlowControl|Delay (Variables|Default|GetSpawn%20Delay))
  (CallFunction|SpawnEnemy3 (Variables|Default|GetTeleport) (Transformation|GetActorTransform) (Variables|Default|GetNumber%20Of%20Enemies)))

(event Custom|SpawnEnemy
  (params (Enemy :type Actor%20Class%20Reference) (SpawnTransform :type Transform) (NumberOfEnemies :type Integer))
  (for _index (range 0 (- NumberOfEnemies 1))
    (Game|SpawnActorfromClass Enemy SpawnTransform "Undefined" 0 0))
  (Utilities|FlowControl|Delay (Variables|Default|GetSpawn%20Delay))
  (CallFunction|SpawnEnemy (Variables|Default|GetEnemy) (Transformation|GetActorTransform) (Variables|Default|GetNumber%20Of%20Enemies)))

(event Custom|SpawnEnemy2
  (params (Take :type Actor%20Class%20Reference) (SpawnTransform :type Transform) (NumberOfEnemies :type Integer))
  (for _index (range 0 (- NumberOfEnemies 1))
    (Game|SpawnActorfromClass Take SpawnTransform "Undefined" 0 0))
  (Utilities|FlowControl|Delay (Variables|Default|GetSpawn%20Delay2))
  (CallFunction|SpawnEnemy2 (Variables|Default|GetTake) (Transformation|GetActorTransform) (Variables|Default|GetNumber%20Of%20Enemies)))

(event EventBeginPlay
  (|CallParentFunction)
  (Utilities|FlowControl|Sequence
    (:then_0
      (CallFunction|SpawnEnemy (Variables|Default|GetEnemy) (Transformation|GetActorTransform) (Variables|Default|GetNumber%20Of%20Enemies)))
    (:then_1
      (CallFunction|SpawnEnemy2 (Variables|Default|GetTake) (Transformation|GetActorTransform) (Variables|Default|GetNumber%20Of%20Enemies)))
    (:then_2
      (CallFunction|SpawnEnemy3 (Variables|Default|GetTeleport) (Transformation|GetActorTransform) (Variables|Default|GetNumber%20Of%20Enemies)))))

(fn ConstructionScript
  (|CallParentFunction))
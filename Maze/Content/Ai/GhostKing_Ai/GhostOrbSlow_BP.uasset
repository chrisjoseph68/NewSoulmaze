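; GhostOrbSlow is an orb actor, filed under the Ghost King AI, that slows the player character on contact.
; Entering its SlowDown component drops ThirdPersonCharacter walk speed to a fixed value, and end overlap sets it to a hardcoded normal speed.
; The orb destroys itself shortly after that contact, or when its lifetime delay from BeginPlay expires.
; A disconnected weapon spawn-and-attach chain never runs.
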(event OnComponentBeginOverlap(SlowDown)
  (params (OverlappedComponent :type Primitive%20Component%20Object%20Reference) (OtherActor :type Actor%20Object%20Reference) (OtherComp :type Primitive%20Component%20Object%20Reference) (OtherBodyIndex :type Integer) (bFromSweep :type Boolean) (SweepResult :type Hit%20Result%20Structure%20%28by%20ref%29))
  (bind _asthird_person_character (Utilities|Casting|CastToThirdPersonCharacter OtherActor))
  (Variables|/Script/Engine.CharacterMovementComponent|SetMaxWalkSpeed (Variables|/Script/Engine.Character|GetCharacterMovement _asthird_person_character) 1.5e+02)
  (Utilities|FlowControl|Delay 2.0)
  (Actor|DestroyActor))

(event OnComponentEndOverlap(SlowDown)
  (params (OverlappedComponent :type Primitive%20Component%20Object%20Reference) (OtherActor :type Actor%20Object%20Reference) (OtherComp :type Primitive%20Component%20Object%20Reference) (OtherBodyIndex :type Integer))
  (bind _asthird_person_character (Utilities|Casting|CastToThirdPersonCharacter OtherActor))
  (Variables|/Script/Engine.CharacterMovementComponent|SetMaxWalkSpeed (Variables|/Script/Engine.Character|GetCharacterMovement _asthird_person_character) 6e+02))

(event EventBeginPlay
  (|CallParentFunction)
  (Utilities|FlowControl|Delay 3e+01)
  (Actor|DestroyActor))

(event Collision|EventActorBeginOverlap
  (params (OtherActor :type Actor%20Object%20Reference))
  ;[1 1 1] Spawn Weapon
)

(fn ConstructionScript
  (|CallParentFunction))
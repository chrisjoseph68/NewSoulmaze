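; Minotaur enemy character that hands its behavior tree and the player pawn to its Minotaur_Ai controller on BeginPlay.
; A looping timer traces down from the right-foot component while velocity X or Y is positive, shaking nearby cameras on ground hits.
; Seeing the player triggers a one-shot timed sound and throttled grunts.
; Overlaps spawn a socket-attached weapon, and EnemyMeleeAttack plays a montage.
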(event OnSeePawn(PawnSensing)
  (params (Pawn :type Pawn%20Object%20Reference))
  (Utilities|Casting|CastToThirdPersonCharacter Pawn)
  (Utilities|FlowControl|Sequence
    (:then_0
      (if (Variables|Default|GetCanseetheplayer?)
        (Utilities|FlowControl|DoOnce false
          (:Completed
            (bind _returnvalue (Audio|SpawnSoundatLocation (Variables|Default|GetSound) (Transformation|GetActorLocation) "0, 0, 0" 1.0 1.0 0.0 0 0))
            (Utilities|FlowControl|Delay 2e+01)
            (Utilities|IsValid _returnvalue
              (:Is%20Valid
                _)))))
      (Audio|Components|Audio|Stop _returnvalue))
    (:then_1
      (Utilities|FlowControl|DoOnce false :!label _label
        (:Completed
          (Audio|SpawnSoundatLocation "/Game/Ai/MinoTaur_Ai/Minator_grunting.Minator_grunting" (Transformation|GetActorLocation) "0, 0, 0" 1.0 1.0 0.0 0 0)
          (Utilities|FlowControl|Delay 6.0)
          (goto _label Reset))))))

(event Custom|FootCheck
  (bind _rfootcheck (Variables|Default|GetRFootCheck))
  (bind _charactermovement (Variables|Character|GetCharacterMovement))
  (bind _returnvalue (Transformation|GetWorldLocation _rfootcheck))
  (bind _velocity (Variables|/Script/Engine.MovementComponent|GetVelocity _charactermovement))
  (if (or (> (.x _velocity) 0.0) (> (.y _velocity) 0.0))
    (bind _outhit (Collision|LineTraceByChannel _returnvalue (+ _returnvalue (* (Transformation|GetActorUpVector) -5e+01)) "TraceTypeQuery1" false 0 "None"))
    (if (.bblockinghit _outhit)
      (Camera|PlayWorldCameraShake "/Game/Ai/MinoTaur_Ai/NewCameraShake.NewCameraShake_C" (Transformation|GetWorldLocation (Variables|Default|GetRFootCheck)) 0.0 1.5e+03 1.0 true))))

(event EventBeginPlay
  (|CallParentFunction)
  (Utilities|FlowControl|Sequence
    (:then_0
      (Utilities|Time|SetTimerbyEvent (delegate Custom|FootCheck) 0.2 true))
    (:then_1
      (bind _asminotaur_ai (Utilities|Casting|CastToMinotaur_Ai (AI|GetAIController self)))
      (Default|SetupAI _asminotaur_ai (Variables|Default|GetBT) (Game|Player|GetPlayerPawn 0)))))

(event EventEnemyMeleeAttack
  ;[1 1 1] MelleAttack
  (Animation|Montage|PlayMontage (Variables|Character|GetMesh) (Variables|Default|GetMontage%20to%20Play)))

(event Collision|EventActorBeginOverlap
  (params (OtherActor :type Actor%20Object%20Reference))
  ;[1 1 1] Spawn Weapon
  (bind _returnvalue (Game|SpawnActorfromClass (Variables|Default|GetClass) (Transformation|GetSocketTransform (Variables|Character|GetMesh) (Variables|Default|GetIn%20Socket%20Name) "RTS_World") "Undefined" 0 0))
  (Transformation|AttachComponentToComponent _returnvalue (Variables|Character|GetMesh) (Variables|Default|GetIn%20Socket%20Name) "SnapToTarget" "SnapToTarget" "SnapToTarget" false))

(fn ConstructionScript
  (|CallParentFunction)
  (Transformation|AttachComponentToComponent (Variables|Default|GetRFootCheck) 0 "Character1_RightFoot" "SnapToTarget" "SnapToTarget" "SnapToTarget" true))